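; Game mode that counts the player's score and records it in a saved high score board.
; AddPoint increments the score.
; On EndPlay it loads the scoreSave slot and copies its entries, using a DoOnce to insert the dated score, named "Player", before the first equal or lower one, or at the end.
; It then saves the list to a new save object and shows it in a ScoreBoard widget.
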(event `self.ReceiveEndPlay`
  (params (EndPlayReason :type "EEndPlayReason Enum" :default "Destroyed"))
  (bind _score (`self.Score`))
  (bind _temp (`self.temp`))
  (bind _returnvalue (`GameplayStatics.LoadGameFromSlot` "scoreSave"))
  (bind _asscore_save (cast `/Game/Blueprints/scoreSave` _returnvalue)
    (:`then`
      (for _array_element (`/Game/Blueprints/scoreSave.playerScores` _asscore_save)
        (`|ExecutionSequence`
          (:`then_0`
            (if (<= (`.score_3_D754408D431FA5BD2145008EB897D74B` (break `/Game/Blueprints/playerScore` _array_element)) _score)
              (`/Engine/EditorBlueprintResources/StandardMacros.DoOnce` false :!label _label
                (:`Completed`
                  (`KismetArrayLibrary.Array_Add` _temp (make `/Game/Blueprints/playerScore` _score (`KismetMathLibrary.GetDate` (struct)) "Player"))))))
          (:`then_1`
            (`KismetArrayLibrary.Array_Add` _temp _array_element))))
      (`|ExecutionSequence`
        (:`then_0`
          (goto _label))
        (:`then_1`
          (bind _returnvalue_2 (`GameplayStatics.CreateSaveGameObject` "/Game/Blueprints/scoreSave.scoreSave_C" :!label _label_2))
          (set `/Game/Blueprints/scoreSave.playerScores` _temp _returnvalue_2)
          (`GameplayStatics.SaveGameToSlot` _returnvalue_2 "scoreSave")
          (bind _returnvalue_3 (`|CreateWidget` "/Game/UI/scoreBoard.scoreBoard_C" null _temp))
          (`UserWidget.AddToViewport` _returnvalue_3 0))))
    (:`CastFailed`
      (`|ExecutionSequence`
        (:`then_0`
          (goto _label))
        (:`then_1`
          (goto _label_2))))))

(fn `addPoint`
  (`/Engine/EditorBlueprintResources/StandardMacros.IncrementInt` (`self.Score`)))

(fn `UserConstructionScript`)