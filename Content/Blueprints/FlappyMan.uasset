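; FlappyMan is the player in a Flappy Bird-style game, driven by physics forces on a capsule.
; The first Jump press enables gravity; each press recreates the score widget and, while alive, applies an impulse-like force, resetting velocity unless moving sideways, and flashes a sprite.
; Tick adds stronger downforce when Jump is released while rising, giving variable jump height.
; "Enemy" overlaps cause a spinning death, then delayed Jump-to-restart; R reloads anytime.
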(event `self.ReceiveBeginPlay`
  (`PrimitiveComponent.SetEnableGravity` (`self.Capsule`) false))

(event `self.Capsule.OnComponentBeginOverlap`
  (params (OverlappedComponent :type "PrimitiveComponent Object Reference") (OtherActor :type "Actor Object Reference") (OtherComp :type "PrimitiveComponent Object Reference") (OtherBodyIndex :type Integer) (bFromSweep :type Boolean) (SweepResult :type "HitResult Structure (by ref)"))
  (`/Engine/EditorBlueprintResources/StandardMacros.IsValid` OtherComp
    (:`Is Valid`
      ;[1 0.076 0] Death Mechanic
      (if (`ActorComponent.ComponentHasTag` OtherComp "Enemy")
        (if (`self.isAlive`)
          (`GameplayStatics.PlaySound2D` "/Game/Sounds/Death.Death" 1.0 1.0 0.0 null null)
          (set `self.isAlive` false)
          (`self.Jump` false)
          (`PrimitiveComponent.AddTorqueInDegrees` (`self.Capsule`) (0.0 -3000000.0 0.0) "None" false)
          (`KismetSystemLibrary.Delay` 1.75)
          (set `self.readyToRestart` true))))))

(event `self.ReceiveTick`
  (params (DeltaSeconds :type "Float (single-precision)"))
  ;[1 1 1] Modified Jump Gravity
  (bind _returnvalue (`PrimitiveComponent.GetPhysicsLinearVelocity` (`self.Capsule`) "None"))
  (if (> (.z _returnvalue) 0.0)
    (if (== (`self.GetInputAxisValue`) 1.0)
      (set `self.DownForce` (* -500.0 DeltaSeconds))
      (else
        (set `self.DownForce` (* -50000.0 DeltaSeconds))))
    (`PrimitiveComponent.AddForce` (`self.Capsule`) (`KismetMathLibrary.MakeVector` 0.0 0.0 (`self.DownForce`)) "None" false)))

(event `InputAction|Jump`
  (params (Key :type "Key Structure"))
  (:`Pressed`
    ;[1 1 1] Jump Mechanic
    (`WidgetLayoutLibrary.RemoveAllWidgets`)
    (bind _returnvalue (`|CreateWidget` "/Game/UI/ScoreInterface.ScoreInterface_C"))
    (`UserWidget.AddToViewport` _returnvalue 0)
    (if (not (`self.isPlaying`))
      (set `self.isPlaying` true)
      (`PrimitiveComponent.SetEnableGravity` (`self.Capsule`) true))
    (if (`self.isAlive`)
      (`GameplayStatics.PlaySound2D` "/Game/Sounds/Jump.Jump" 1.0 1.0 0.0 null null)
      (`self.Jump` (or (== (`self.GetInputAxisValue`) 1.0) (== (`self.GetInputAxisValue`) 1.0)))
      (elif (`self.readyToRestart`)
        (`GameplayStatics.OpenLevel` "FlappyLevel" :!label _label)))))

(event `Key|R`
  (params (Key :type "Key Structure"))
  ;[1 1 1] Jump Mechanic
  (:`Pressed`
    (goto _label)))

(event `InputAction|Jump`
  (params (Key :type "Key Structure"))
  (:`Pressed`
    ;[1 1 1] Jump Animation
    (if (`self.isAlive`)
      (`PaperSpriteComponent.SetSprite` (`self.PaperSprite`) "/Game/Sprites/SpriteSheet3_Sprite_1.SpriteSheet3_Sprite_1")
      (`KismetSystemLibrary.Delay` 0.2)
      (`PaperSpriteComponent.SetSprite` (`self.PaperSprite`) "/Game/Sprites/SpriteSheet3_Sprite_0.SpriteSheet3_Sprite_0"))))

(event `InputAction|Move Left`
  (params (Key :type "Key Structure"))
  (:`Pressed`
    ;[1 1 1] Move Left
    (if (`self.isPlaying`)
      (`PrimitiveComponent.AddForce` (`self.Capsule`) (-10000.0 0.0 0.0) "None" false)
      (`SceneComponent.K2_SetWorldRotation` (`self.Capsule`) (struct :`Yaw` 180.0) false false))))

(event `InputAction|Move Right`
  (params (Key :type "Key Structure"))
  (:`Pressed`
    ;[1 1 1] Move Right
    (if (`self.isPlaying`)
      (`PrimitiveComponent.AddForce` (`self.Capsule`) (10000.0 0.0 0.0) "None" false)
      (`SceneComponent.K2_SetWorldRotation` (`self.Capsule`) (struct :`Yaw` 360.0) false false))))

(fn `Jump`
  (params (bAddToCurrent :type Boolean))
  (`PrimitiveComponent.SetPhysicsLinearVelocity` (`self.Capsule`) (0.0 0.0 0.0) bAddToCurrent "None")
  (`PrimitiveComponent.AddForce` (`self.Capsule`) (0.0 0.0 20000.0) "None" false))

(fn `UserConstructionScript`)