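; Block is an obstacle actor, labeled as logs, that carries a collectible coin and scrolls down the world Z axis.
; BeginPlay shifts it by a random X offset, and Tick moves it at a constant delta-time-scaled speed while yawing the coin each frame.
; Overlapping the coin adds a point through BP_GameMode, plays a sound and destroys the coin component, leaving the block moving.
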(event `self.ReceiveBeginPlay`
  (`SceneComponent.K2_SetWorldLocation` (`self.DefaultSceneRoot`) (+ (`SceneComponent.K2_GetComponentLocation` (`self.DefaultSceneRoot`)) (`KismetMathLibrary.MakeVector` (`KismetMathLibrary.RandomFloatInRange` -1000.0 1000.0))) false false))

(event `self.Coin.OnComponentBeginOverlap`
  (params (OverlappedComponent :type "PrimitiveComponent Object Reference") (OtherActor :type "Actor Object Reference") (OtherComp :type "PrimitiveComponent Object Reference") (OtherBodyIndex :type Integer) (bFromSweep :type Boolean) (SweepResult :type "HitResult Structure (by ref)"))
  ;[0.1779 1 0.07128] Point Mechanic
  (bind _asbp_game_mode (cast `/Game/BP_GameMode` (`GameplayStatics.GetGameMode`)))
  (`/Game/BP_GameMode.addPoint` _asbp_game_mode)
  (`GameplayStatics.PlaySound2D` "/Game/Sounds/Coin.Coin" 1.0 1.0 0.0 null null)
  (`ActorComponent.K2_DestroyComponent` (`self.Coin`)))

(event `self.ReceiveTick`
  (params (DeltaSeconds :type "Float (single-precision)"))
  (bind _coin (`self.Coin`))
  (bind _returnvalue (`SceneComponent.K2_GetComponentRotation` _coin))
  ;[1 1 1] Move Logs
  (`SceneComponent.K2_SetWorldLocation` (`self.DefaultSceneRoot`) (+ (`SceneComponent.K2_GetComponentLocation` (`self.DefaultSceneRoot`)) (`KismetMathLibrary.MakeVector` 0.0 0.0 (* DeltaSeconds -500.0))) false false)
  (`/Engine/EditorBlueprintResources/StandardMacros.IsValid` _coin
    (:`Is Valid`
      ;[1 1 1] Coin Rotating Mechanic
      (`SceneComponent.K2_SetWorldRotation` _coin (`KismetMathLibrary.RInterpTo` _returnvalue (`KismetMathLibrary.MakeRotator` 0.0 0.0 (+ (.yaw _returnvalue) 2.5)) (`GameplayStatics.GetWorldDeltaSeconds`)) false false))))

(fn `UserConstructionScript`)