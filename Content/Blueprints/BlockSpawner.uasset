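; BlockSpawner is an actor that repeatedly spawns Block actors at its own transform while the player's FlappyMan pawn is playing.
; BeginPlay caches the pawn, then Tick checks IsPlaying and plays a timeline that updates SpawnSpeed.
; Each timeline update feeds SpawnSpeed into a Delay before spawning, so the pending Delay throttles updates into a spawn interval that varies along the curve.
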(event `self.ReceiveBeginPlay`
  (bind _asflappy_man (cast `/Game/Blueprints/FlappyMan` (`GameplayStatics.GetPlayerPawn` 0))
    (:`then`
      (set `self.Player` _asflappy_man))
    (:`CastFailed`
      (`KismetSystemLibrary.PrintString` "Could not convert player pawn to Flappy Jones"))))

(event `self.ReceiveTick`
  (params (DeltaSeconds :type "Float (single-precision)"))
  (if (`/Game/Blueprints/FlappyMan.isPlaying` (`self.Player`))
    ;[1 1 1] Increment Spawn Speed
    (bind (_direction _spawnspeed) (`Timeline|Timeline_0`)
      (:`Update`
        (bind _output_get (set `self.spawnSpeed` _spawnspeed))
        (`KismetSystemLibrary.Delay` _output_get)
        (`|SpawnActorFromClass` "/Game/Blueprints/Block.Block_C" (`SceneComponent.K2_GetComponentToWorld` (`self.DefaultSceneRoot`)) "Undefined" "OverrideRootScale" null null)))))

(fn `UserConstructionScript`)